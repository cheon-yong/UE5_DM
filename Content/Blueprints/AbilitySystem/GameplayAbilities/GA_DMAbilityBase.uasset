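; Base gameplay ability that runs a cast-then-montage flow for the player character.
; With a positive CastingTime, it snaps the character to face the cursor's ground-plane direction, registers itself with the controller, stops auto-run and holds the Casting state for that duration.
; It then restores Living and plays a fixed cast montage, ending on completion; instant casts go straight to the montage.
; The target-data facing path through CombatInterface is unconnected.
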(event `self.K2_ActivateAbility`
  (if (> (`self.CastingTime`) 0.0)
    (bind _asbp_dmcharacter (`self.BPCasting`))
    (`AbilityTask_WaitDelay.WaitDelay` (`self.CastingTime`)
      (:`OnFinish`
        (`DMCharacter.SetCharacterState` _asbp_dmcharacter "Living"))))
  (`AbilityTask_PlayMontageAndWait.CreatePlayMontageAndWaitProxy` "None" "/Game/Blueprints/Animations/Shinbi/Animations/Combat/Ability_AttackWolves_Cast_L2_Montage.Ability_AttackWolves_Cast_L2_Montage"
    (:`OnCompleted`
      (`self.K2_EndAbility`))))

(fn `BPCasting`
  (returns (`AsBP DMCharacter` :type "/Game/Blueprints/Character/BP_DMCharacter Object Reference"))
  (bind _returnvalue (`self.GetAvatarActorFromActorInfo`))
  (bind _asbp_dmcharacter (cast `/Game/Blueprints/Character/BP_DMCharacter` _returnvalue))
  (bind _asbp_player_controller (cast `/Game/Blueprints/Controller/BP_PlayerController` (`Pawn.GetController` _asbp_dmcharacter)))
  (`self.LookAtMousePoint` _asbp_player_controller _returnvalue)
  (`DMPlayerController.SetActivatingAbility` _asbp_player_controller self)
  (set `DMPlayerController.bAutoRunning` false _asbp_player_controller)
  (`DMCharacter.SetCharacterState` _asbp_dmcharacter "Casting")
  (return _asbp_dmcharacter))

(fn `LookAtMousePoint`
  (params (PlayerController :type "PlayerController Object Reference") (Actor :type "Actor Object Reference"))
  (bind (_returnvalue_x _returnvalue_y) (`KismetMathLibrary.BreakVector` (- (`.Location` (`GameplayStatics.BreakHitResult` (`PlayerController.GetHitResultUnderCursorByChannel` PlayerController "TraceTypeQuery1" true))) (`Actor.K2_GetActorLocation` Actor))))
  (`Actor.K2_SetActorRotation` Actor (`KismetMathLibrary.RInterpTo` (`Actor.K2_GetActorRotation` Actor) (`KismetMathLibrary.Conv_VectorToRotator` (`KismetMathLibrary.MakeVector` _returnvalue_x _returnvalue_y)) (`GameplayStatics.GetWorldDeltaSeconds`) 0.0) false))

(fn `UpdateFacing`
  (params (HitResult :type "GameplayAbilityTargetDataHandle Structure (by ref)"))
  (bind _output_get (set `self.Location` (`.Location` (`GameplayStatics.BreakHitResult` (`AbilitySystemBlueprintLibrary.GetHitResultFromTargetData` HitResult)))))
  (bind _ascombat_interface (cast `CombatInterface` (`self.GetAvatarActorFromActorInfo`)))
  (`CombatInterface.UpdateFacingTarget` _ascombat_interface _output_get))