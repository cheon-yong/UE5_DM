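; Gameplay ability for Shinbi's plain attack, a three-step montage combo that spawns a projectile toward the point under the mouse.
; On activation it gets cursor target data, turns the avatar to face that location, and picks the montage from BP_DMCharacter's ComboAttack index.
; All branches share a wait for the FireBolt montage event, which spawns the projectile and ends the ability; montage interruption also ends it.
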(event `self.K2_ActivateAbility`
  (bind (_asynctaskproxy _datahandle) (`TargetDataUnderMouse.CreateTargetDataUnderMouse`)
    (:`ValidData`
      (set `self.Location` (`.Location` (`GameplayStatics.BreakHitResult` (`AbilitySystemBlueprintLibrary.GetHitResultFromTargetData` _datahandle))))
      (bind _ascombat_interface (cast `CombatInterface` (`self.GetAvatarActorFromActorInfo`)))
      (`CombatInterface.UpdateFacingTarget` _ascombat_interface (`self.Location`))
      (bind _asbp_dmcharacter (cast `/Game/Blueprints/Character/BP_DMCharacter` (`self.GetAvatarActorFromActorInfo`)))
      (bind _combo (`/Game/Blueprints/Character/BP_DMCharacter.ComboAttack` _asbp_dmcharacter))
      (switch `int` _combo
        (:`0`
          (`AbilityTask_PlayMontageAndWait.CreatePlayMontageAndWaitProxy` "None" "/Game/Blueprints/Animations/Shinbi/Animations/Combat/PrimaryMelee_D_Slow_Montage.PrimaryMelee_D_Slow_Montage"
            (:`then`
              (`AbilityTask_WaitGameplayEvent.WaitGameplayEvent` (struct :`TagName` "Event.Montage.FireBolt") null :!label _label
                (:`EventReceived`
                  (`self.SpawnProjectile` (`self.Location`))
                  (`self.K2_EndAbility`))))
            (:`OnInterrupted`
              (`self.K2_EndAbility` :!label _label_2))))
        (:`1`
          (`AbilityTask_PlayMontageAndWait.CreatePlayMontageAndWaitProxy` "None" "/Game/Blueprints/Animations/Shinbi/Animations/Combat/PrimaryMelee_B_Slow_Montage.PrimaryMelee_B_Slow_Montage"
            (:`then`
              (goto _label))
            (:`OnInterrupted`
              (goto _label_2))))
        (:`2`
          (`AbilityTask_PlayMontageAndWait.CreatePlayMontageAndWaitProxy` "None" "/Game/Blueprints/Animations/Shinbi/Animations/Combat/PrimaryMelee_C_Slow2_Montage.PrimaryMelee_C_Slow2_Montage"
            (:`then`
              (goto _label))
            (:`OnInterrupted`
              (goto _label_2))))))))