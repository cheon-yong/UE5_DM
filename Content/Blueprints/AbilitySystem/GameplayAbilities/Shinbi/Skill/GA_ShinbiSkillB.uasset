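; Gameplay ability for Shinbi's Skill B that handles the targeting stage by spawning a BP_SkillArea cursor.
; On activation it checks player controller 0 for an already activating ability and only prints a message if one exists.
; Otherwise it spawns the cursor at the world origin and registers itself on the controller as the activating ability.
; Ending the ability destroys the cursor; no skill effect is applied here.
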(event `self.K2_OnEndAbility`
  (params (bWasCancelled :type Boolean))
  (`/Engine/EditorBlueprintResources/StandardMacros.IsValid` (`self.Cursor`)
    (:`Is Valid`
      (`Actor.K2_DestroyActor` (`self.Cursor`)))))

(event `self.K2_ActivateAbility`
  (bind _asbp_player_controller (cast `/Game/Blueprints/Controller/BP_PlayerController` (`GameplayStatics.GetPlayerController` 0)))
  (bind _returnvalue (`DMPlayerController.GetActivatingAbility` _asbp_player_controller))
  (`/Engine/EditorBlueprintResources/StandardMacros.IsValid` _returnvalue
    (:`Is Valid`
      (`KismetSystemLibrary.PrintString` "Already Activating"))
    (:`Is Not Valid`
      (bind _returnvalue_2 (`|SpawnActorFromClass` "/Game/Blueprints/Actor/Area/BP_SkillArea.BP_SkillArea_C" (`KismetMathLibrary.MakeTransform` (0.0 0.0 0.0)) "Undefined" "MultiplyWithRoot" null null))
      (set `self.Cursor` _returnvalue_2)
      (bind _asbp_player_controller_2 (cast `/Game/Blueprints/Controller/BP_PlayerController` (`GameplayStatics.GetPlayerController` 0)))
      (`DMPlayerController.SetActivatingAbility` _asbp_player_controller_2 self))))