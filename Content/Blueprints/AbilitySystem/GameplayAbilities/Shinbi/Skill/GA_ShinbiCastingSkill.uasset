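; Shinbi gameplay ability that runs a casting skill aimed at the point under the mouse.
; On valid target data it updates facing, then, if a casting time is set, enters casting and waits before restoring the Living state.
; It then plays the wolves attack cast montage, immediately for zero cast time, and ends only when the montage completes.
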(event `self.K2_ActivateAbility`
  (bind (_asynctaskproxy _datahandle) (`TargetDataUnderMouse.CreateTargetDataUnderMouse`)
    (:`ValidData`
      (`self.UpdateFacing` _datahandle)
      (if (> (`self.CastingTime`) 0.0)
        (bind _asbp_dmcharacter (`self.BPCasting`))
        (`AbilityTask_WaitDelay.WaitDelay` (`self.CastingTime`)
          (:`OnFinish`
            (`DMCharacter.SetCharacterState` _asbp_dmcharacter "Living"))))
      (`AbilityTask_PlayMontageAndWait.CreatePlayMontageAndWaitProxy` "None" "/Game/Blueprints/Animations/Shinbi/Animations/Combat/Ability_AttackWolves_Cast_L2_Montage.Ability_AttackWolves_Cast_L2_Montage"
        (:`OnCompleted`
          (`self.K2_EndAbility`))))))