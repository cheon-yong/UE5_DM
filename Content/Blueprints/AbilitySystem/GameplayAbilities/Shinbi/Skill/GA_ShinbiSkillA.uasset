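; GA_ShinbiSkillA is Shinbi's gameplay ability for an aimed projectile skill with a targeting cursor.
; Activation creates a BP_SkillArea cursor, which is destroyed when the ability ends.
; ContinueAbility takes the location under the mouse, turns the avatar toward it via CombatInterface and plays the wolf-attack cast montage.
; The montage's projectile gameplay event spawns the projectile toward that location and ends the ability.
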(event `self.K2_OnEndAbility`
  (params (bWasCancelled :type Boolean))
  (`/Engine/EditorBlueprintResources/StandardMacros.IsValid` (`self.Cursor`)
    (:`Is Valid`
      (`Actor.K2_DestroyActor` (`self.Cursor`)))))

(event `self.K2_ActivateAbility`
  (bind _returnvalue (`self.CreateCursor`))
  (`/Engine/EditorBlueprintResources/StandardMacros.IsValid` _returnvalue
    (:`Is Valid`
      (bind _asbp_skill_area (cast `/Game/Blueprints/Actor/Area/BP_SkillArea` _returnvalue))
      (set `self.Cursor` _asbp_skill_area))
    (:`Is Not Valid`
      (`KismetSystemLibrary.PrintString` "Already"))))

(event `self.ContinueAbility`
  (bind (_asynctaskproxy _datahandle) (`TargetDataUnderMouse.CreateTargetDataUnderMouse`)
    (:`ValidData`
      (bind _output_get (set `self.Location` (`.Location` (`GameplayStatics.BreakHitResult` (`AbilitySystemBlueprintLibrary.GetHitResultFromTargetData` _datahandle)))))
      (bind _ascombat_interface (cast `CombatInterface` (`self.GetAvatarActorFromActorInfo`))
        (:`then`
          (`CombatInterface.UpdateFacingTarget` _ascombat_interface _output_get)
          (bind _asbp_dmcharacter (cast `/Game/Blueprints/Character/BP_DMCharacter` (`self.GetAvatarActorFromActorInfo`)))
          (`|PlayMontage` (`Character.Mesh` _asbp_dmcharacter) "/Game/Blueprints/Animations/Shinbi/Animations/Combat/Ability_AttackWolves_Cast_L2_Montage.Ability_AttackWolves_Cast_L2_Montage"
            (:`then`
              (`AbilityTask_WaitGameplayEvent.WaitGameplayEvent` (struct :`TagName` "Event.Montage.Projectile") null
                (:`then`
                  (`self.SpawnProjectile` (`self.Location`) false)
                  (`self.K2_EndAbility`))))))
        (:`CastFailed`
          (`KismetSystemLibrary.PrintString` "Cast Failed"))))))