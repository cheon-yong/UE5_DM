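; BP_DMCharacter_Origin is a character Blueprint with helpers for facing a target and tracking a melee-style attack combo.
; UpdateFacingTarget writes a location into the Motion Warping "FacingTarget" warp target, so warped animations can orient toward it.
; ComboAttack increments the Combo counter, wraps it to zero past a small limit, and returns it.
; ResetCombo zeroes the counter and prints it for debugging.
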(event `CombatInterface.UpdateFacingTarget`
  (params (Target :type "Vector Structure (by ref)"))
  (`MotionWarpingComponent.AddOrUpdateWarpTargetFromLocation` (`self.MotionWarping`) "FacingTarget" Target))

(event `ResetCombo`
  (bind _output_get (set `self.Combo` 0))
  (`KismetSystemLibrary.PrintString` (`KismetTextLibrary.Conv_TextToString` (`|FormatText` "Combo {0}" _output_get))))

(fn `ComboAttack`
  (returns (Combo :type Integer))
  (bind _result (`/Engine/EditorBlueprintResources/StandardMacros.IncrementInt` (`self.Combo`))
    (:`  `
      (if (> _result 2)
        (set `self.Combo` 0)
        (else
          (set `self.Combo` _result)))
      (return (`self.Combo`)))))

(fn `UserConstructionScript`)