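; Character Blueprint that provides a three-hit melee combo and a motion-warping facing target.
; PlainAttack switches on the Combo counter to advance it cyclically and play the matching slow primary melee montage, while ResetCombo returns it to zero.
; UpdateFacingTarget feeds a location into the MotionWarping component as the FacingTarget warp point.
; Combo changes in both attack and reset print the counter as debug text.
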(event `PlainAttack`
  (switch `int` (`self.Combo`)
    (:`0`
      (set `self.Combo` 1)
      (`self.PrintCombo`)
      (`self.PlayAnimMontage` "/Game/Blueprints/Animations/Shinbi/Animations/Combat/PrimaryMelee_B_Slow_Montage.PrimaryMelee_B_Slow_Montage"))
    (:`1`
      (set `self.Combo` 2)
      (`self.PrintCombo`)
      (`self.PlayAnimMontage` "/Game/Blueprints/Animations/Shinbi/Animations/Combat/PrimaryMelee_C_Slow2_Montage.PrimaryMelee_C_Slow2_Montage"))
    (:`2`
      (set `self.Combo` 0)
      (`self.PrintCombo`)
      (`self.PlayAnimMontage` "/Game/Blueprints/Animations/Shinbi/Animations/Combat/PrimaryMelee_D_Slow_Montage.PrimaryMelee_D_Slow_Montage"))))

(event `CombatInterface.UpdateFacingTarget`
  (params (Target :type "Vector Structure (by ref)"))
  (`MotionWarpingComponent.AddOrUpdateWarpTargetFromLocation` (`self.MotionWarping`) "FacingTarget" Target))

(event `ResetCombo`
  (bind _output_get (set `self.Combo` 0))
  (`KismetSystemLibrary.PrintString` (`KismetTextLibrary.Conv_TextToString` (`|FormatText` "Combo {0}" _output_get))))

(fn `PrintCombo`
  (`KismetSystemLibrary.PrintString` (`KismetTextLibrary.Conv_TextToString` (`|FormatText` "Combo {0}" (`self.Combo`)))))

(fn `UserConstructionScript`)