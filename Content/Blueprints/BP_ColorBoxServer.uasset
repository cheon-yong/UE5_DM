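; BP_ColorBoxServer is a networking test box that changes to a random color when a locally controlled pawn enters its color area.
; Only remote clients pick the color, then pass it to ChangeColorServer, which stores BoxColor and tints a dynamic material.
; A second area sets the overlapping actor as owner on the authority, as client-to-server RPCs require.
; OnRep_BoxColor applies replicated color changes to the material.
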(event `self.ReceiveBeginPlay`
  (bind _returnvalue (`PrimitiveComponent.CreateDynamicMaterialInstance` (`self.Mesh`) 0 "/Game/Blueprints/Materials/M_Color.M_Color" "None"))
  (bind _output_get (set `self.MI_Color` _returnvalue))
  (`PrimitiveComponent.SetMaterial` (`self.Mesh`) 0 _output_get))

(event `ChangeToRandomColor`
  (`/Engine/EditorBlueprintResources/ActorMacros.Switch Has Authority`
    (:`Remote`
      (bind _output_get (set `self.BoxColor` (`KismetMathLibrary.MakeColor` (`KismetMathLibrary.RandomFloatInRange` 0.0 1.0) (`KismetMathLibrary.RandomFloatInRange` 0.0 1.0) (`KismetMathLibrary.RandomFloatInRange` 0.0 1.0))))
      (`self.ChangeColorServer` _output_get))))

(event `ChangeColorServer`
  (params (NewColor :type "LinearColor Structure"))
  (bind _output_get (set `self.BoxColor` NewColor))
  (`MaterialInstanceDynamic.SetVectorParameterValue` (`self.MI_Color`) "Color" _output_get))

(event `self.ChangeColorArea.OnComponentBeginOverlap`
  (params (OverlappedComponent :type "PrimitiveComponent Object Reference") (OtherActor :type "Actor Object Reference") (OtherComp :type "PrimitiveComponent Object Reference") (OtherBodyIndex :type Integer) (bFromSweep :type Boolean) (SweepResult :type "HitResult Structure (by ref)"))
  (bind _aspawn (cast `Pawn` OtherActor))
  (if (`Pawn.IsLocallyControlled` _aspawn)
    (`self.ChangeToRandomColor`)))

(event `self.ChangeOwnerArea.OnComponentBeginOverlap`
  (params (OverlappedComponent :type "PrimitiveComponent Object Reference") (OtherActor :type "Actor Object Reference") (OtherComp :type "PrimitiveComponent Object Reference") (OtherBodyIndex :type Integer) (bFromSweep :type Boolean) (SweepResult :type "HitResult Structure (by ref)"))
  (`/Engine/EditorBlueprintResources/ActorMacros.Switch Has Authority`
    (:`Authority`
      (`self.SetOwner` OtherActor))))

(fn `OnRep_BoxColor`
  (`MaterialInstanceDynamic.SetVectorParameterValue` (`self.MI_Color`) "Color" (`self.BoxColor`)))

(fn `UserConstructionScript`)